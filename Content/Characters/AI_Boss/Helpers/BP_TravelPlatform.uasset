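; BP_TravelPlatform is an AI boss helper actor: a platform that sinks when triggered and then removes itself.
; MovePlatformDown plays a timeline that lerps the Cube's relative location toward one unit below its current position on each update, so the descent accumulates per tick.
; When the timeline finishes, it destroys the referenced travel point actor along with the platform.
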(event `self.ReceiveBeginPlay`
  (set `self.PlatformRef` self))

(event `MovePlatformDown`
  (bind _relativelocation (`SceneComponent.RelativeLocation` (`/Game/Characters/AI_Boss/Helpers/BP_TravelPlatform.Cube` (`self.PlatformRef`))))
  (bind (_direction _platformtransform) (`Timeline|Timeline`)
    (:`Update`
      (`SceneComponent.K2_SetRelativeLocation` (`self.Cube`) (`KismetMathLibrary.VLerp` _relativelocation (- _relativelocation (0.0 0.0 1.0)) _platformtransform) false false))
    (:`Finished`
      (`self.K2_DestroyActor` (`self.TravelPointRef`))
      (`self.K2_DestroyActor`))))

(fn `UserConstructionScript`)
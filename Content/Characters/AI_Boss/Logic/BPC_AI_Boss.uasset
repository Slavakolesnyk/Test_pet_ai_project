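; AI Controller for the boss, running its behavior tree and writing state, enemy and spawn data to the Blackboard.
; Server-side perception fills a player target map that sets Enemy, with a second, toggleable sight component working around stale sight updates.
; Looping timers record peak target count and gate minion spawning on minion, player and travel-platform counts.
; It also spawns minions at the boss's hand and calls existing ones back to it.
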(event `MinionsIntoBossHand`
  (bind _asbp_aiboss (cast `/Game/Characters/AI_Boss/BP_AIBoss` (`self.K2_GetPawn`)))
  (bind _outactors (`GameplayStatics.GetAllActorsOfClass` "/Game/Characters/AI_Minion/BP_AIMinion.BP_AIMinion_C"))
  (for _array_element _outactors
    (bind _asbpc_ai_miniion (cast `/Game/Characters/AI_Minion/Logic/BPC_AI_Miniion` (`Pawn.GetController` _array_element)))
    (bind _asbpc_ai_boss (cast `/Game/Characters/AI_Boss/Logic/BPC_AI_Boss` (`Pawn.GetController` _asbp_aiboss)))
    (`/Game/Characters/AI_Minion/Logic/BPC_AI_Miniion.BossCallsYou` _asbpc_ai_miniion _array_element (`SceneComponent.GetSocketLocation` (`Character.Mesh` _asbp_aiboss) "LeftHand_Socket") _asbpc_ai_boss)))

(event `self.ReceiveBeginPlay`
  (`self.RunBehaviorTree` "/Game/Characters/AI_Boss/Logic/BT/BT/BT_AI_Boss.BT_AI_Boss"))

(event `CalculatePlatforms`
  (bind _returnvalue (`AIBlueprintHelperLibrary.GetBlackboard` null))
  ;[1 1 1] Reasons to spawn/Not
  (bind _outactors (`GameplayStatics.GetAllActorsOfClass` "/Game/Characters/AI_Minion/BP_AIMinion.BP_AIMinion_C"))
  (bind _outactors_2 (`GameplayStatics.GetAllActorsOfClass` "/Game/ThirdPerson/Blueprints/BP_Player.BP_Player_C"))
  (bind _outactors_3 (`GameplayStatics.GetAllActorsOfClass` "/Game/Characters/AI_Boss/Helpers/BP_TravelPlatform.BP_TravelPlatform_C"))
  (bind _returnvalue_2 (== (`KismetArrayLibrary.Array_Length` _outactors_3) 0))
  (if _returnvalue_2
    (`BlackboardComponent.SetValueAsBool` _returnvalue "NoPointsAlive" true))
  (if (or (>= (`KismetArrayLibrary.Array_Length` _outactors) (+ (`KismetArrayLibrary.Array_Length` _outactors_2) 1)) _returnvalue_2)
    (`BlackboardComponent.SetValueAsBool` _returnvalue "ShouldMinionToSpawn" false)
    (else
      (`BlackboardComponent.SetValueAsBool` _returnvalue "ShouldMinionToSpawn" true))))

(event `self.ReceivePossess`
  (params (PossessedPawn :type "Pawn Object Reference"))
  (set `self.BossREF` PossessedPawn)
  (set `self.BossStates` "NewEnumerator2")
  (`KismetSystemLibrary.K2_SetTimerDelegate` (delegate `CalculateTargets`) 1.5 true)
  (`KismetSystemLibrary.K2_SetTimerDelegate` (delegate `CalculatePlatforms`) 1.5 true))

(event `CalculateTargets`
  (bind _currenttargetamount (`self.CurrentTargetAmount`))
  ;[1 0.1446 0.1248] Targets
  (set `self.CurrentTargetAmount` (`BlueprintMapLibrary.Map_Length` (`self.MapofTargets`)))
  (if (and (>= _currenttargetamount 0) (<= (`self.MaxTargetAmount`) _currenttargetamount))
    (bind _output_get (set `self.MaxTargetAmount` _currenttargetamount))
    (`BlackboardComponent.SetValueAsInt` (`AIBlueprintHelperLibrary.GetBlackboard` null) "EnemiesInFight" _output_get)))

(event `SpawnMinion`
  (bind _returnvalue (`BlackboardComponent.GetValueAsClass` (`AIBlueprintHelperLibrary.GetBlackboard` null) "MinionNext"))
  ;[0.2604 0.2604 0.2604] Spawn minions
  (switch `int` (`KismetMathLibrary.RandomIntegerInRange` 0 2)
    (:`0`
      (set `self.DiviationToSpawn` (20.0 20.0 20.0)))
    (:`1`
      (set `self.DiviationToSpawn` (80.0 80.0 60.0)))
    (:`2`
      (set `self.DiviationToSpawn` (135.0 135.0 50.0)))
    (:`3`
      (set `self.DiviationToSpawn` (170.0 170.0 20.0))))
  (if (`KismetSystemLibrary.IsValidClass` _returnvalue)
    (bind _asbp_aiboss (cast `/Game/Characters/AI_Boss/BP_AIBoss` (`self.BossREF`)))
    (bind _asactor (castclass `Actor` _returnvalue))
    (set `self.MinonClass` _asactor)
    (bind (_returnvalue_location _returnvalue_rotation _returnvalue_scale) (`KismetMathLibrary.BreakTransform` (`SceneComponent.GetSocketTransform` (`Character.Mesh` _asbp_aiboss) "ik_hand_lSocket" "RTS_World")))
    (`|SpawnActorFromClass` (`self.MinonClass`) (`KismetMathLibrary.MakeTransform` (+ _returnvalue_location (`self.DiviationToSpawn`)) (struct) _returnvalue_scale) "AlwaysSpawn" "MultiplyWithRoot" self self)))

(event `self.AIPerception_SightUpdated.OnTargetPerceptionInfoUpdated`
  (params (UpdateInfo :type "ActorPerceptionUpdateInfo Structure (by ref)"))
  ;[1 0 0.8812] Need to avoid Unreal issue with non updated sight, called from BT Service of AI
  (`/Engine/EditorBlueprintResources/ActorMacros.Switch Has Authority`
    (:`Authority`
      (if (== (`GameplayStatics.GetObjectClass` UpdateInfo_Target) "/Game/ThirdPerson/Blueprints/BP_Player.BP_Player_C")
        (`self.SetEnemy` UpdateInfo_Target UpdateInfo_TargetId (`.bSuccessfullySensed` (break `AIStimulus` UpdateInfo_Stimulus)))
        (`self.CheckStatus`)
        (else
          (`self.CheckStatus`))))))

(event `self.AIPerception.OnTargetPerceptionInfoUpdated`
  (params (UpdateInfo :type "ActorPerceptionUpdateInfo Structure (by ref)"))
  (bind (_age _expirationage _strength _stimuluslocation _receiverlocation _tag _bsuccessfullysensed) (break `AIStimulus` UpdateInfo_Stimulus))
  ;[0.8231 0.4259 1] Senses
  (`/Engine/EditorBlueprintResources/ActorMacros.Switch Has Authority`
    (:`Authority`
      (if _bsuccessfullysensed
        (if (== (`GameplayStatics.GetObjectClass` UpdateInfo_Target) "/Game/ThirdPerson/Blueprints/BP_Player.BP_Player_C")
          (bind _returnvalue (`AIPerceptionSystem.GetSenseClassForStimulus` UpdateInfo_Stimulus))
          (switch `string` (`KismetSystemLibrary.GetClassDisplayName` _returnvalue)
            (:`AISense_Sight`
              (`self.SetEnemy` UpdateInfo_Target UpdateInfo_TargetId _bsuccessfullysensed)
              (`self.CheckStatus`))))))))

(fn `CallSightSenseUpdate`
  (params (isActivated :type Boolean))
  (`AIPerceptionComponent.SetSenseEnabled` (`self.AIPerception_SightUpdated`) "/Script/AIModule.AISense_Sight" isActivated))

(fn `CheckStatus`
  (locals (TempDistanceTarget :type "Float (double-precision)") (TempTargetsIDremove :type "Array of Integer") (TempEnemy :type "Actor Object Reference"))
  (bind _mapoftargets (`self.MapofTargets`))
  (`/Engine/EditorBlueprintResources/StandardMacros.IsValid` (`self.K2_GetPawn`)
    (:`Is Valid`
      (bind _keys (`BlueprintMapLibrary.Map_Keys` _mapoftargets))
      (bind _values (`BlueprintMapLibrary.Map_Values` _mapoftargets))
      (for (_array_element _array_index) _values
        (`/Engine/EditorBlueprintResources/StandardMacros.IsValid` _array_element
          (:`Is Valid`
            (if (`self.Visible`)
              (if (`KismetSystemLibrary.IsValid` (`local.TempEnemy`))
                (bind _returnvalue (`self.GetSquaredDistanceTo` _array_element (`local.TempEnemy`)))
                (if (< _returnvalue (`local.TempDistanceTarget`))
                  (set `local.TempEnemy` _array_element :!label _label)
                  (set `local.TempDistanceTarget` _returnvalue))
                (else
                  (goto _label)))
              (else
                (`KismetArrayLibrary.Array_AddUnique` (`local.TempTargetsIDremove`) (`|GetArrayItem` _keys _array_index) :!label _label_2))))
          (:`Is Not Valid`
            (goto _label_2))))
      (for _array_element_2 (`local.TempTargetsIDremove`)
        (`BlueprintMapLibrary.Map_Remove` (`self.MapofTargets`) _array_element_2))
      ;[1 1 1] to fix
      (`self.TempEnemySet` (`local.TempEnemy`))
      (`/Engine/EditorBlueprintResources/StandardMacros.IsValid` (`local.TempEnemy`)
        (:`Is Valid`
          (return))))))

(fn `MakeBossAttack`
  (if (`|EnumInequality` (`self.BossStates`) "NewEnumerator3")
    (bind _output_get (set `self.BossStates` "NewEnumerator3"))
    (`self.Set States in BB` _output_get)
    (return)))

(fn `MakeBossRestoreHP`
  (if (`|EnumInequality` (`self.BossStates`) "NewEnumerator1")
    (bind _output_get (set `self.BossStates` "NewEnumerator1"))
    (`self.Set States in BB` _output_get)
    (return)))

(fn `MakeBossSpawn`
  (if (`|EnumInequality` (`self.BossStates`) "NewEnumerator0")
    (bind _output_get (set `self.BossStates` "NewEnumerator0"))
    (`self.Set States in BB` _output_get)
    (return)))

(fn `MakeBossTravel`
  (if (`|EnumInequality` (`self.BossStates`) "NewEnumerator2")
    (bind _output_get (set `self.BossStates` "NewEnumerator2"))
    (`self.Set States in BB` _output_get)
    (return)))

(fn `RemoveTarget`
  (locals (TempDistancearget :type "Float (double-precision)") (TempTargetsIDremove :type "Array of Integer") (TempEnemy :type "Actor Object Reference"))
  (`BlackboardComponent.ClearValue` (`self.Blackboard`) "Enemy"))

(fn `Set States in BB`
  (params (State :type "/Game/Characters/AI_Boss/Helpers/BossStates Enum" :default "NewEnumerator0"))
  (`BlackboardComponent.SetValueAsEnum` (`AIBlueprintHelperLibrary.GetBlackboard` null) "States" State)
  (return))

(fn `SetEnemy`
  (params (ActorTarget :type "Actor Object Reference") (IDtarget :type Integer) (Visible :type Boolean))
  (set `self.Visible` Visible)
  (`/Engine/EditorBlueprintResources/StandardMacros.IsValid` ActorTarget
    (:`Is Valid`
      (if (`self.Visible`)
        (if (`.ReturnValue` (`BlueprintMapLibrary.Map_Find` (`self.MapofTargets`) IDtarget))
          (return)
          (else
            (`BlueprintMapLibrary.Map_Add` (`self.MapofTargets`) IDtarget ActorTarget)
            (return)))
        (else
          _)))
    (:`Is Not Valid`
      _))
  (`self.RemoveTarget`)
  (`self.CheckStatus`))

(fn `TempEnemySet`
  (params (TempEnemy :type "Actor Object Reference"))
  (locals (Temptarget :type "Actor Object Reference"))
  (`/Engine/EditorBlueprintResources/StandardMacros.IsValid` TempEnemy
    (:`Is Valid`
      (`BlackboardComponent.SetValueAsObject` (`self.Blackboard`) "Enemy" TempEnemy)
      (return))
    (:`Is Not Valid`
      (`self.RemoveTarget`))))

(fn `UserConstructionScript`)
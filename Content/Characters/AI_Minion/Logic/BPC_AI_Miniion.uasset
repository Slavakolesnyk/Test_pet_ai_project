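; AI controller for boss-callable minions, running BT_AIMinion and supplying random patrol points.
; Server-side sight and hearing update target and stimulus data, from which CheckStatus sets Blackboard enemy and Neutral/Alert/Combat state, toggling minion visibility.
; A second, toggleable sight perception works around Unreal's stale-sight issue.
; BossCallsYou stops AI logic, then timelines lift, spin and move the minion to a location, destroy it and notify the boss controller.
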(event `self.ReceiveTick`
  (params (DeltaSeconds :type "Float (single-precision)"))
  (set `self.Delta Seconds` DeltaSeconds))

(event `FindPatrollRandomPoint`
  (bind _aiminionref (`self.aiMinionREF`))
  ;[0 1 0.6724] Actions
  (`/Engine/EditorBlueprintResources/StandardMacros.IsValid` _aiminionref
    (:`Is Valid`
      (set `self.PatrolPoint` (`NavigationSystemV1.K2_GetRandomReachablePointInRadius` (`self.K2_GetActorLocation` _aiminionref) 900.0 null null))
      (`self.SetPatrolPoint`))))

(event `MoveMinionsToBoss`
  ;[0 1 0.6724] Actions
  (bind (_direction _newtrack_0) (`Timeline|MoveToBossTimeline` :!via `PlayFromStart`)
    (:`Update`
      (`self.K2_SetActorLocation` (stale `BossCallsYou` MinionPawn) (`KismetMathLibrary.VLerp` (`self.K2_GetActorLocation` (stale `BossCallsYou` MinionPawn)) (stale `BossCallsYou` LocationMoveTo) _newtrack_0) false false))
    (:`Finished`
      (`self.K2_DestroyActor` (stale `BossCallsYou` MinionPawn))
      (`/Game/Characters/AI_Boss/Logic/BPC_AI_Boss.BossGainMinions` (stale `BossCallsYou` BossController)))))

(event `BossCallsYou`
  (params (MinionPawn :type "/Game/Characters/AI_Minion/BP_AIMinion Object Reference") (LocationMoveTo :type "Vector Structure") (BossController :type "/Game/Characters/AI_Boss/Logic/BPC_AI_Boss Object Reference"))
  (bind (_returnvalue_x _returnvalue_y _returnvalue_z) (`KismetMathLibrary.BreakVector` (`self.K2_GetActorLocation` MinionPawn)))
  (bind _charactermovement (`Character.CharacterMovement` MinionPawn))
  (bind (_returnvalue_roll _returnvalue_pitch _returnvalue_yaw) (`KismetMathLibrary.BreakRotator` (`CharacterMovementComponent.GetLastUpdateRotation` _charactermovement)))
  ;[0 1 0.6724] Actions
  (`/Game/Characters/AI_Minion/BP_AIMinion.MakeMinionVisible` MinionPawn)
  (`BrainComponent.StopLogic` (`self.BrainComponent`) "")
  (`CharacterMovementComponent.SetMovementMode` (`Character.CharacterMovement` MinionPawn) "MOVE_None" 0)
  (bind (_direction _curveup) (`Timeline|GoUpTimeline` :!via `PlayFromStart`)
    (:`Update`
      (`self.K2_SetActorLocation` MinionPawn (`KismetMathLibrary.MakeVector` _returnvalue_x _returnvalue_y (+ _returnvalue_z _curveup)) false false)
      (set `CharacterMovementComponent.bOrientRotationToMovement` false _charactermovement)
      (bind (_direction_2 _newtrack_0) (`Timeline|MinionRotationTimeline` :!via `PlayFromStart`)
        (:`Update`
          (bind _returnvalue (* (+ _newtrack_0 _returnvalue_yaw) (`self.Delta Seconds`)))
          (`self.K2_AddActorWorldRotation` MinionPawn (`KismetMathLibrary.MakeRotator` _returnvalue _returnvalue) false false)
          (`KismetSystemLibrary.K2_SetTimerDelegate` (delegate `MoveMinionsToBoss`) 1.75))))))

(event `self.ReceiveBeginPlay`
  ;[0.9895 1 0.2725] Main
  (`self.RunBehaviorTree` "/Game/Characters/AI_Minion/Logic/BT/BT_AIMinion.BT_AIMinion"))

(event `self.ReceivePossess`
  (params (PossessedPawn :type "Pawn Object Reference"))
  ;[0.9895 1 0.2725] Main
  (bind _asbp_aiminion (cast `/Game/Characters/AI_Minion/BP_AIMinion` PossessedPawn))
  (set `self.aiMinionREF` _asbp_aiminion)
  (bind _output_get (set `self.CurrentMentalState` "NewEnumerator0"))
  (`self.SetCharSpeed` _output_get))

(event `OnDestroyed_Event`
  (params (DestroyedActor :type "Actor Object Reference"))
  ;[0.9895 1 0.2725] Main
  (`BrainComponent.StopLogic` (`self.BrainComponent`) "Death"))

(event `self.AIPerception.OnTargetPerceptionInfoUpdated`
  (params (UpdateInfo :type "ActorPerceptionUpdateInfo Structure (by ref)"))
  (bind (_age _expirationage _strength _stimuluslocation _receiverlocation _tag _bsuccessfullysensed) (break `AIStimulus` UpdateInfo_Stimulus))
  ;[0.8231 0.4259 1] Senses
  (`/Engine/EditorBlueprintResources/ActorMacros.Switch Has Authority`
    (:`Authority`
      (if (== (`GameplayStatics.GetObjectClass` UpdateInfo_Target) "/Game/ThirdPerson/Blueprints/BP_Player.BP_Player_C")
        (if _bsuccessfullysensed
          (bind _returnvalue (`AIPerceptionSystem.GetSenseClassForStimulus` UpdateInfo_Stimulus))
          (switch `string` (`KismetSystemLibrary.GetClassDisplayName` _returnvalue)
            (:`AISense_Sight`
              (`self.SetEnemy` UpdateInfo_Target UpdateInfo_TargetId _bsuccessfullysensed))
            (:`AISense_Hearing`
              (`self.SetStimul` _stimuluslocation)))
          (else
            (`self.SetEnemy` null 0 _bsuccessfullysensed)
            (`self.SetStimul` _stimuluslocation)
            (`KismetSystemLibrary.K2_SetTimerDelegate` (delegate `ForgetAboutLastSeenPosition`) 6.0)))
        (`self.CheckStatus` :!label _label)))))

(event `ForgetAboutLastSeenPosition`
  ;[0.8231 0.4259 1] Senses
  (`BlackboardComponent.ClearValue` (`AIBlueprintHelperLibrary.GetBlackboard` null) "StimulusLocation")
  (goto _label))

(event `self.AIPerception_SightUpdated.OnTargetPerceptionInfoUpdated`
  (params (UpdateInfo :type "ActorPerceptionUpdateInfo Structure (by ref)"))
  (bind (_age _expirationage _strength _stimuluslocation _receiverlocation _tag _bsuccessfullysensed) (break `AIStimulus` UpdateInfo_Stimulus))
  ;[1 0 0.8812] Need to avoid Unreal issue with non updated sight, called from BT Service of AI
  (`/Engine/EditorBlueprintResources/ActorMacros.Switch Has Authority`
    (:`Authority`
      (if (== (`GameplayStatics.GetObjectClass` UpdateInfo_Target) "/Game/ThirdPerson/Blueprints/BP_Player.BP_Player_C")
        (`self.SetEnemy` UpdateInfo_Target UpdateInfo_TargetId _bsuccessfullysensed)
        (if (== _bsuccessfullysensed false)
          (`self.SetStimul` _stimuluslocation)
          (`self.CheckStatus`)
          (else
            (`self.CheckStatus`)))))))

(fn `CallSightSenseUpdate`
  (params (isActivated :type Boolean))
  (`AIPerceptionComponent.SetSenseEnabled` (`self.AIPerception_SightUpdated`) "/Script/AIModule.AISense_Sight" isActivated))

(fn `CheckStatus`
  (locals (TempDistanceTarget :type "Float (double-precision)") (TempTargetsIDremove :type "Array of Integer") (TempEnemy :type "Actor Object Reference"))
  (bind _mapoftargets (`self.MapofTargets`))
  (`/Engine/EditorBlueprintResources/StandardMacros.IsValid` (`self.K2_GetPawn`)
    (:`Is Valid`
      (bind _keys (`BlueprintMapLibrary.Map_Keys` _mapoftargets))
      (bind _values (`BlueprintMapLibrary.Map_Values` _mapoftargets))
      (for (_array_element _array_index) _values
        (`/Engine/EditorBlueprintResources/StandardMacros.IsValid` _array_element
          (:`Is Valid`
            (if (`self.Visible`)
              (if (`KismetSystemLibrary.IsValid` (`local.TempEnemy`))
                (bind _asactor (cast `Actor` (`BlackboardComponent.GetValueAsObject` (`AIBlueprintHelperLibrary.GetBlackboard` null) "enemy")))
                (if (< (stale _output_get) (`self.GetSquaredDistanceTo` _asactor self))
                  (`KismetSystemLibrary.PrintString` "TRUE" true true (struct :`R` 0.128574 :`G` 1.0 :`A` 1.0) 1.0)
                  (set `local.TempEnemy` _array_element :!label _label)
                  (bind _output_get (set `local.TempDistanceTarget` (`self.GetSquaredDistanceTo` (`local.TempEnemy`))))
                  (else
                    (`KismetSystemLibrary.PrintString` "False" true true (struct :`R` 1.0 :`B` 0.133678 :`A` 1.0) 1.0)))
                (else
                  (goto _label)))
              (else
                (`KismetArrayLibrary.Array_AddUnique` (`local.TempTargetsIDremove`) (`|GetArrayItem` _keys _array_index) :!label _label_2))))
          (:`Is Not Valid`
            (goto _label_2))))
      (for _array_element_2 (`local.TempTargetsIDremove`)
        (`BlueprintMapLibrary.Map_Remove` (`self.MapofTargets`) _array_element_2))
      (`self.TempEnemySet` (`local.TempEnemy`))
      (`/Engine/EditorBlueprintResources/StandardMacros.IsValid` (`local.TempEnemy`)
        (:`Is Valid`
          (`self.StartCombat`)
          (return))
        (:`Is Not Valid`
          (if (`BlackboardComponent.IsVectorValueSet` (`self.Blackboard`) "StimulusLocation")
            (`self.StartAlert`)
            (return)
            (else
              (`self.StartNeutral`)
              (return))))))))

(fn `GenAlert`
  (`self.StartNeutral`))

(fn `RemoveTarget`
  (`BlackboardComponent.ClearValue` (`self.Blackboard`) "Enemy"))

(fn `Set Mental States in BB`
  (`BlackboardComponent.SetValueAsEnum` (`self.Blackboard`) "MentalState" (`self.CurrentMentalState`))
  (return))

(fn `SetCharSpeed`
  (params (MentalState :type "/Game/Characters/AI_Minion/Helpers/Enums/MentalStates Enum" :default "NewEnumerator0"))
  (bind _ascharacter (cast `Character` (`self.aiMinionREF`)))
  (switch `/Game/Characters/AI_Minion/Helpers/Enums/MentalStates` MentalState
    (:`NewEnumerator0`
      (set `self.Max Walk Speed` 400.0))
    (:`NewEnumerator1`
      (set `self.Max Walk Speed` 425.0))
    (:`NewEnumerator2`
      (set `self.Max Walk Speed` 450.0)))
  (set `CharacterMovementComponent.MaxWalkSpeed` (`self.Max Walk Speed`) (`Character.CharacterMovement` _ascharacter)))

(fn `SetEnemy`
  (params (ActorTarget :type "Actor Object Reference") (IDtarget :type Integer) (Visible :type Boolean))
  (set `self.Visible` Visible)
  (`/Engine/EditorBlueprintResources/StandardMacros.IsValid` ActorTarget
    (:`Is Valid`
      (if (`self.Visible`)
        (if (`.ReturnValue` (`BlueprintMapLibrary.Map_Find` (`self.MapofTargets`) IDtarget))
          (return)
          (else
            (`BlueprintMapLibrary.Map_Add` (`self.MapofTargets`) IDtarget ActorTarget)
            (return)))
        (else
          _)))
    (:`Is Not Valid`
      _))
  (`self.RemoveTarget`)
  (`self.CheckStatus`))

(fn `SetPatrolPoint`
  (bind _patrolpoint (`self.PatrolPoint`))
  (if (`AIBlueprintHelperLibrary.IsValidAILocation` (`self.PatrolPoint`))
    (`BlackboardComponent.SetValueAsVector` (`self.Blackboard`) "RandomPointPatrolling" _patrolpoint)
    (`KismetSystemLibrary.DrawDebugBox` _patrolpoint (0.0 0.0 0.0) (struct :`R` 1.0 :`B` 0.500774 :`A` 1.0) (struct) 5.0 100.0)
    (return)))

(fn `SetStimul`
  (params (Stimul :type "Vector Structure"))
  (locals (StimulusLocation :type "Vector Structure"))
  (set `local.StimulusLocation` Stimul)
  (`BlackboardComponent.SetValueAsVector` (`self.Blackboard`) "StimulusLocation" (`local.StimulusLocation`)))

(fn `StartAlert`
  (if (`|EnumInequality` (`self.CurrentMentalState`) "NewEnumerator1")
    (set `self.CurrentMentalState` "NewEnumerator1")
    (`self.Set Mental States in BB`)
    (bind _asbp_aiminion (cast `/Game/Characters/AI_Minion/BP_AIMinion` (`self.K2_GetPawn`)))
    (`/Game/Characters/AI_Minion/BP_AIMinion.MakeMinionVisible` _asbp_aiminion)
    (return)))

(fn `StartCombat`
  (if (`|EnumInequality` (`self.CurrentMentalState`) "NewEnumerator2")
    (set `self.CurrentMentalState` "NewEnumerator2")
    (`self.Set Mental States in BB`)
    (bind _asbp_aiminion (cast `/Game/Characters/AI_Minion/BP_AIMinion` (`self.K2_GetPawn`)))
    (`/Game/Characters/AI_Minion/BP_AIMinion.MakeMinionVisible` _asbp_aiminion)
    (return)))

(fn `StartNeutral`
  (if (`|EnumInequality` (`self.CurrentMentalState`) "NewEnumerator0")
    (set `self.CurrentMentalState` "NewEnumerator0")
    (`self.Set Mental States in BB`)
    (bind _asbp_aiminion (cast `/Game/Characters/AI_Minion/BP_AIMinion` (`self.K2_GetPawn`)))
    (`/Game/Characters/AI_Minion/BP_AIMinion.MakeMinionInvisible` _asbp_aiminion)
    (return)))

(fn `TempEnemySet`
  (params (TempEnemy :type "Actor Object Reference"))
  (locals (Temptarget :type "Actor Object Reference"))
  (`/Engine/EditorBlueprintResources/StandardMacros.IsValid` TempEnemy
    (:`Is Valid`
      (`BlackboardComponent.SetValueAsObject` (`self.Blackboard`) "Enemy" TempEnemy)
      (return))
    (:`Is Not Valid`
      (`self.RemoveTarget`))))

(fn `UserConstructionScript`)
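; BP_HealItem is a health pickup that heals the player on contact and then removes itself.
; A capsule overlap with an actor of exactly the BP_Player class calls NotifyAndAction, which runs HealAndDestroy.
; That function sends RegenerateHPMessage to the player with a fixed heal amount and destroys the item.
; The item's own HP and damage functions are stubs returning zero or false.
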(event `self.ReceiveBeginPlay`)

(event `self.Capsule.OnComponentBeginOverlap`
  (params (OverlappedComponent :type "PrimitiveComponent Object Reference") (OtherActor :type "Actor Object Reference") (OtherComp :type "PrimitiveComponent Object Reference") (OtherBodyIndex :type Integer) (bFromSweep :type Boolean) (SweepResult :type "HitResult Structure (by ref)"))
  (if (== (`GameplayStatics.GetObjectClass` OtherActor) "/Game/ThirdPerson/Blueprints/BP_Player.BP_Player_C")
    (`self.NotifyAndAction` OtherActor)))

(event `NotifyAndAction`
  (params (Actor :type "Actor Object Reference"))
  (`self.HealAndDestroy` Actor))

(fn `ApplyDamageHP`
  (params (DamageInfo :type "/Game/Interfaces/Attribute/Struct_DamageINFO Structure"))
  (returns (WasDamaged :type Boolean))
  (return false))

(fn `GetCurrentHP`
  (returns (Health :type "Float (double-precision)"))
  (return 0.0))

(fn `GetMaxHP`
  (returns (MaxHP :type "Float (double-precision)"))
  (return 0.0))

(fn `HealAndDestroy`
  (params (Target :type "Actor Object Reference"))
  (message `/Game/Interfaces/Attribute/BP_Atrtribute_Interface.RegenerateHP` Target 10.0)
  (`self.K2_DestroyActor`))

(fn `RegenerateHP`
  (params (AmountRecoverHP :type "Float (double-precision)"))
  (returns (NewHP :type "Float (double-precision)"))
  (return 0.0))

(fn `UserConstructionScript`)
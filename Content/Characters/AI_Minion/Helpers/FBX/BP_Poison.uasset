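; BP_Poison is a timed poison explosive actor that deals area damage and destroys itself.
; BeginPlay starts a 4.5-second timer, presumably for AOE_PoisonDamage, which skips detonation if its attribute component reports dead.
; Detonation spawns an explosion effect, plays a sound at world origin and runs a debug-drawn sphere trace for pawns.
; Only the single hit actor receives damage, through an ApplyDamageHP message.
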(event `self.ReceiveBeginPlay`
  (bind _returnvalue (`KismetSystemLibrary.K2_SetTimerDelegate` (`|CreateDelegate` :!event `AOE_PoisonDamage`) 4.5))
  (set `self.BoomTImer` _returnvalue))

(event `AOE_PoisonDamage`
  (bind _returnvalue (`self.K2_GetActorLocation`))
  (if (not (`/Game/Interfaces/Attribute/BPC_Attributesystem.IsDead` (`self.BPC_Attributesystem`)))
    (`GameplayStatics.SpawnEmitterAtLocation` "/Game/StarterContent/Particles/P_Explosion.P_Explosion" _returnvalue)
    (`GameplayStatics.PlaySoundAtLocation` "/Game/StarterContent/Audio/Explosion02.Explosion02" (0.0 0.0 0.0) (struct) 1.0 1.0 0.0 null null null null)
    (bind (_outhit _returnvalue_2) (`KismetSystemLibrary.SphereTraceSingleForObjects` :`Start` _returnvalue :`End` (+ _returnvalue (0.0 0.0 200.0)) :`Radius` 350.0 :`ObjectTypes` (`|MakeArray` "ObjectTypeQuery3" :!type "EObjectTypeQuery Enum") :`DrawDebugType` "ForDuration" :`DrawTime` 1.0))
    (if _returnvalue_2
      (message `/Game/Interfaces/Attribute/BP_Atrtribute_Interface.ApplyDamageHP` (`.HitActor` (`GameplayStatics.BreakHitResult` _outhit)) (make `/Game/Interfaces/Attribute/Struct_DamageINFO` 25.0 false false "NewEnumerator1" "NewEnumerator3")))
    (`self.K2_DestroyActor`)))

(fn `UserConstructionScript`)
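; Base projectile actor that flies toward an assigned target and damages players on impact.
; Shortly after spawn, a timer sets its velocity once toward the target's location at max speed, so it does not keep homing.
; The collision box ignores the owner; a hit calls CallProjectileHit, plays impact effect and sound, applies fixed damage through a message if the hit actor is BP_Player, then destroys the projectile.
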(event `RotateProjectile`
  (set `MovementComponent.Velocity` (* (`KismetMathLibrary.GetDirectionUnitVector` (`self.K2_GetActorLocation`) (`self.K2_GetActorLocation` (`self.ProjectileTarget`))) (`self.MaxSpeed`)) (`self.ProjectileMovement`)))

(event `self.ReceiveBeginPlay`
  (`PrimitiveComponent.IgnoreActorWhenMoving` (`self.Box`) (`self.GetOwner`) true)
  (set `ProjectileMovementComponent.MaxSpeed` (`self.MaxSpeed`) (`self.ProjectileMovement`))
  (`KismetSystemLibrary.K2_SetTimerDelegate` (delegate `WaitUntilProjectileSpawned`) 0.05))

(event `WaitUntilProjectileSpawned`
  (`self.ProjectileTarget`
    (:`then`
      (`self.RotateProjectile`))
    (:`else`)))

(event `self.Box.OnComponentHit`
  (params (HitComponent :type "PrimitiveComponent Object Reference") (OtherActor :type "Actor Object Reference") (OtherComp :type "PrimitiveComponent Object Reference") (NormalImpulse :type "Vector Structure") (Hit :type "HitResult Structure (by ref)"))
  (bind (_bblockinghit _binitialoverlap _time _distance _location _impactpoint _normal _impactnormal _physmat _hitactor) (`GameplayStatics.BreakHitResult` Hit))
  (`self.ProjectileHit` OtherActor Hit)
  (bind _asbp_player (cast `/Game/ThirdPerson/Blueprints/BP_Player` _hitactor)
    (:`then`
      (`self.Projectile_overlapped` _location _asbp_player true))
    (:`CastFailed`
      (`self.Projectile_overlapped` _location))))

(event `Projectile_overlapped`
  (params (HitLocation :type "Vector Structure") (Actor :type "/Game/ThirdPerson/Blueprints/BP_Player Object Reference") (Player :type Boolean))
  (`GameplayStatics.SpawnEmitterAtLocation` (`self.EffectOnHit`) HitLocation)
  (`GameplayStatics.PlaySoundAtLocation` (`self.SoundOnHit`) HitLocation (struct) 1.0 1.0 0.0 null null null null)
  (if Player
    (message `/Game/Interfaces/Attribute/BP_Atrtribute_Interface.ApplyDamageHP` Actor (make `/Game/Interfaces/Attribute/Struct_DamageINFO` 25.0 false false "NewEnumerator2" "NewEnumerator2")))
  (`self.K2_DestroyActor`))

(fn `UserConstructionScript`)
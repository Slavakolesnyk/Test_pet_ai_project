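; BPC_Attributesystem is an attribute component that manages a character's HP, healing, damage and death.
; Heal adds HP clamped between zero and the maximum, and both Heal and DealDamage act only while alive.
; DealDamage takes a damage info struct, lets blocking cancel blockable hits, otherwise subtracts HP.
; Dispatcher-style calls signal blocks, death and hit reactions, the latter when the hit forces interruption or the character is interruptible.
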(fn `Deal Damage`
  (params (DamageInfo :type "/Game/Interfaces/Attribute/Struct_DamageINFO Structure"))
  (returns (WasDamaged :type Boolean))
  (bind (_amount _canbeblocked _shouldinterupt _damagereaction) (break `/Game/Interfaces/Attribute/Struct_DamageINFO` DamageInfo))
  (if (not (`self.IsDead`))
    (if (and (`self.IsBlocking`) _canbeblocked)
      (`self.OnDamageBlocked`)
      (return false)
      (else
        (bind _output_get (set `self.CurrentHP` (- (`self.CurrentHP`) _amount)))
        (if (<= _output_get 0.0)
          (set `self.IsDead` true)
          (`self.OnCharDeath`)
          (return true)
          (elif (or _shouldinterupt (`self.IsInterrupbtable`))
            (`self.OnDamageReact` _damagereaction)
            (return true)))))))

(fn `Heal`
  (params (AmountHealHP :type "Float (double-precision)"))
  (returns (NewHP :type "Float (double-precision)"))
  (if (not (`self.IsDead`))
    (bind _output_get (set `self.CurrentHP` (`KismetMathLibrary.FClamp` (+ AmountHealHP (`self.CurrentHP`)) 0.0 (`self.MaxHP`))))
    (return _output_get)))
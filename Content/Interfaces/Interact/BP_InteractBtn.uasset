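; BP_InteractBtn is a button that the player triggers by overlapping its box, sending a linked travel platform down.
; The overlap starts the MoveBTN timeline, which nudges the button mesh slightly downward from its current relative location on each update, so the offset accumulates.
; When the timeline finishes, it casts the owner reference to BP_TravelPlatform and calls MovePlatformDown.
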(event `self.Box.OnComponentBeginOverlap`
  (params (OverlappedComponent :type "PrimitiveComponent Object Reference") (OtherActor :type "Actor Object Reference") (OtherComp :type "PrimitiveComponent Object Reference") (OtherBodyIndex :type Integer) (bFromSweep :type Boolean) (SweepResult :type "HitResult Structure (by ref)"))
  (cast `/Game/ThirdPerson/Blueprints/BP_Player` OtherActor)
  (`self.MoveButton`))

(event `MoveButton`
  (bind _relativelocation (`SceneComponent.RelativeLocation` (`self.InteractBTN`)))
  (bind (_direction _buttontransform) (`Timeline|MoveBTN`)
    (:`Update`
      (`SceneComponent.K2_SetRelativeLocation` (`self.InteractBTN`) (`KismetMathLibrary.VLerp` _relativelocation (- _relativelocation (0.0 0.0 0.1)) _buttontransform) false false))
    (:`Finished`
      (bind _asbp_travel_platform (cast `/Game/Characters/AI_Boss/Helpers/BP_TravelPlatform` (`self.ButtonOnwerRef`)))
      (`/Game/Characters/AI_Boss/Helpers/BP_TravelPlatform.MovePlatformDown` _asbp_travel_platform))))

(fn `UserConstructionScript`)
(event `self.ReceiveBeginPlay`
  (`self.RunBehaviorTree` "/Game/Characters/AI_Boss/Logic/BT/BT/BT_AI_Boss.BT_AI_Boss"))

(event `self.ReceivePossess`
  (params (PossessedPawn :type "Pawn Object Reference"))
  (set `self.BossREF` PossessedPawn)
  (set `self.BossStates` "NewEnumerator0"))

(fn `MakeBossAttack`
  (if (`|EnumInequality` (`self.BossStates`) "NewEnumerator3")
    (set `self.BossStates` "NewEnumerator3")
    (`self.Set States in BB`)
    (return)))

(fn `MakeBossRestoreHP`
  (if (`|EnumInequality` (`self.BossStates`) "NewEnumerator1")
    (set `self.BossStates` "NewEnumerator1")
    (`self.Set States in BB`)
    (return)))

(fn `MakeBossSpawn`
  (if (`|EnumInequality` (`self.BossStates`) "NewEnumerator0")
    (set `self.BossStates` "NewEnumerator0")
    (`self.Set States in BB`)
    (return)))

(fn `MakeBossTravel`
  (if (`|EnumInequality` (`self.BossStates`) "NewEnumerator2")
    (set `self.BossStates` "NewEnumerator2")
    (`self.Set States in BB`)
    (return)))

(fn `Set States in BB`
  (`BlackboardComponent.SetValueAsEnum` (`self.Blackboard`) "States" (`self.BossStates`))
  (return))

(fn `UserConstructionScript`)
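; AI controller for the minion: runs BT_AIMinion and forwards health calls to an attribute component, calling a heal-item spawn on damage.
; Authority-only perception records sighted players and heard player locations.
; CheckStatus prunes invalid targets, picks an enemy by squared distance, and writes it to the Blackboard alongside stimulus and random patrol points.
; StartCombat, StartAlert and StartNeutral all assign Neutral, so Combat and Alert are never set.
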(event `Controller_spawn`
  (bind (_returnvalue_x _returnvalue_y _returnvalue_z) (`KismetMathLibrary.BreakVector` (`SceneComponent.K2_GetComponentLocation` (`Actor.RootComponent` (`self.aiMinionREF`)))))
  (`|SpawnActorFromClass` "/Game/Characters/AI_Minion/Helpers/HealItem/BP_HealItem.BP_HealItem_C" (`KismetMathLibrary.MakeTransform` (`KismetMathLibrary.MakeVector` _returnvalue_x (+ _returnvalue_y 350.0) (+ _returnvalue_z 220.0))) "AlwaysSpawn" "MultiplyWithRoot" null null))

(event `self.ReceiveBeginPlay`
  ;[1 0.848 0.8079] Main
  (`self.RunBehaviorTree` "/Game/Characters/AI_Minion/Logic/BT/BT_AIMinion.BT_AIMinion"))

(event `self.ReceivePossess`
  (params (PossessedPawn :type "Pawn Object Reference"))
  ;[1 0.848 0.8079] Main
  (`/Engine/EditorBlueprintResources/ActorMacros.Switch Has Authority`
    (:`Authority`
      (set `self.aiMinionREF` PossessedPawn)
      (bind _output_get (set `self.CurrentMentalState` "NewEnumerator0"))
      (`self.SetCharSpeed` _output_get))))

(event `self.ReceiveUnPossess`
  (params (UnpossessedPawn :type "Pawn Object Reference"))
  ;[1 0.848 0.8079] Main
)

(event `OnDestroyed_Event`
  (params (DestroyedActor :type "Actor Object Reference"))
  ;[1 0.848 0.8079] Main
  (`BrainComponent.StopLogic` (`self.BrainComponent`) "Death"))

(event `FindPatrollRandomPoint`
  (bind _aiminionref (`self.aiMinionREF`))
  ;[0 1 0.6724] Actions
  (`/Engine/EditorBlueprintResources/StandardMacros.IsValid` _aiminionref
    (:`Is Valid`
      (set `self.PatrolPoint` (`NavigationSystemV1.K2_GetRandomReachablePointInRadius` (`self.K2_GetActorLocation` _aiminionref) 900.0 null null))
      (`self.SetPatrolPoint`))))

(event `self.AIPerception.OnTargetPerceptionInfoUpdated`
  (params (UpdateInfo :type "ActorPerceptionUpdateInfo Structure (by ref)"))
  (bind (_age _expirationage _strength _stimuluslocation _receiverlocation _tag _bsuccessfullysensed) (break `AIStimulus` UpdateInfo_Stimulus))
  ;[0.8231 0.4259 1] Senses
  (`/Engine/EditorBlueprintResources/ActorMacros.Switch Has Authority`
    (:`Authority`
      (if _bsuccessfullysensed
        (if (== (`GameplayStatics.GetObjectClass` UpdateInfo_Target) "/Game/ThirdPerson/Blueprints/BP_Player.BP_Player_C")
          (bind _returnvalue (`AIPerceptionSystem.GetSenseClassForStimulus` UpdateInfo_Stimulus))
          (switch `string` (`KismetSystemLibrary.GetClassDisplayName` _returnvalue)
            (:`AISense_Sight`
              (`self.SetEnemy` UpdateInfo_Target UpdateInfo_TargetId)
              (`self.CheckStatus`))
            (:`AISense_Hearing`
              (`self.SetStimul` _stimuluslocation)
              (`self.CheckStatus`))))))))

(fn `ApplyDamageHP`
  (params (DamageInfo :type "/Game/AttributeSystem/Struct_DamageINFO Structure"))
  (returns (WasDamaged :type Boolean))
  (bind _wasdamaged (`/Game/AttributeSystem/BPC_Attributesystem.TakeDamage` (`self.BPC_Attributesystem`) DamageInfo))
  (`self.Controller_spawn`)
  (return _wasdamaged))

(fn `CheckStatus`
  (locals (TempDistanceTarget :type "Float (double-precision)") (TempTargetsIDremove :type "Array of Integer") (TempEnemy :type "Actor Object Reference"))
  (bind _mapoftargets (`self.MapofTargets`))
  (`/Engine/EditorBlueprintResources/StandardMacros.IsValid` (`self.K2_GetPawn`)
    (:`Is Valid`
      (bind _keys (`BlueprintMapLibrary.Map_Keys` _mapoftargets))
      (bind _values (`BlueprintMapLibrary.Map_Values` _mapoftargets))
      (for (_array_element _array_index) _values
        (`/Engine/EditorBlueprintResources/StandardMacros.IsValid` _array_element
          (:`Is Valid`
            (if (`KismetSystemLibrary.IsValid` (`local.TempEnemy`))
              (bind _returnvalue (`self.GetSquaredDistanceTo` _array_element (`local.TempEnemy`)))
              (if (< _returnvalue (`local.TempDistanceTarget`))
                (set `local.TempEnemy` _array_element :!label _label)
                (set `local.TempDistanceTarget` _returnvalue))
              (else
                (goto _label))))
          (:`Is Not Valid`
            (`KismetArrayLibrary.Array_AddUnique` (`local.TempTargetsIDremove`) (`|GetArrayItem` _keys _array_index)))))
      (for _array_element_2 (`local.TempTargetsIDremove`)
        (`BlueprintMapLibrary.Map_Remove` (`self.MapofTargets`) _array_element_2))
      (`self.TempEnemySet` (`local.TempEnemy`))
      (`/Engine/EditorBlueprintResources/StandardMacros.IsValid` (`local.TempEnemy`)
        (:`Is Valid`
          (`self.StartCombat`)
          (return))
        (:`Is Not Valid`
          (if (`BlackboardComponent.IsVectorValueSet` (`self.Blackboard`) "StimulusLocation")
            (`self.StartAlert`)
            (return)
            (else
              (`self.StartNeutral`)
              (return))))))))

(fn `GetCurrentHP`
  (returns (Health :type "Float (double-precision)"))
  (return (`/Game/AttributeSystem/BPC_Attributesystem.CurrentHP` (`self.BPC_Attributesystem`))))

(fn `GetMaxHP`
  (returns (MaxHP :type "Float (double-precision)"))
  (return (`/Game/AttributeSystem/BPC_Attributesystem.MaxHP` (`self.BPC_Attributesystem`))))

(fn `RegenerateHP`
  (params (AmountRecoverHP :type "Float (double-precision)"))
  (returns (NewHP :type "Float (double-precision)"))
  (bind _newhp (`/Game/AttributeSystem/BPC_Attributesystem.Heal` (`self.BPC_Attributesystem`) AmountRecoverHP))
  (return _newhp))

(fn `RemoveTarget`
  (`BlackboardComponent.ClearValue` (`self.Blackboard`) "Enemy"))

(fn `Set Mental States in BB`
  (`BlackboardComponent.SetValueAsEnum` (`self.Blackboard`) "MentalState" (`self.CurrentMentalState`))
  (return))

(fn `SetCharSpeed`
  (params (MentalState :type "/Game/Characters/AI_Minion/Helpers/Enums/MentalStates Enum" :default "NewEnumerator0"))
  (bind _ascharacter (cast `Character` (`self.aiMinionREF`)))
  (switch `/Game/Characters/AI_Minion/Helpers/Enums/MentalStates` MentalState
    (:`NewEnumerator0`
      (set `self.Max Walk Speed` 400.0))
    (:`NewEnumerator1`
      (set `self.Max Walk Speed` 425.0))
    (:`NewEnumerator2`
      (set `self.Max Walk Speed` 450.0)))
  (set `CharacterMovementComponent.MaxWalkSpeed` (`self.Max Walk Speed`) (`Character.CharacterMovement` _ascharacter)))

(fn `SetEnemy`
  (params (ActorTarget :type "Actor Object Reference") (IDtarget :type Integer))
  (`/Engine/EditorBlueprintResources/StandardMacros.IsValid` ActorTarget
    (:`Is Valid`
      (if (`.ReturnValue` (`BlueprintMapLibrary.Map_Find` (`self.MapofTargets`) IDtarget))
        (return)
        (else
          (`BlueprintMapLibrary.Map_Add` (`self.MapofTargets`) IDtarget ActorTarget)
          (return))))
    (:`Is Not Valid`
      (`self.RemoveTarget`))))

(fn `SetPatrolPoint`
  (bind _patrolpoint (`self.PatrolPoint`))
  (if (`AIBlueprintHelperLibrary.IsValidAILocation` (`self.PatrolPoint`))
    (`BlackboardComponent.SetValueAsVector` (`self.Blackboard`) "RandomPointPatrolling" _patrolpoint)
    (`KismetSystemLibrary.DrawDebugBox` _patrolpoint (0.0 0.0 0.0) (struct :`R` 1.0 :`B` 0.500774 :`A` 1.0) (struct) 5.0 100.0)
    (return)))

(fn `SetStimul`
  (params (Stimul :type "Vector Structure"))
  (locals (StimulusLocation :type "Vector Structure"))
  (set `local.StimulusLocation` Stimul)
  (`BlackboardComponent.SetValueAsVector` (`self.Blackboard`) "StimulusLocation" (`local.StimulusLocation`)))

(fn `StartAlert`
  (if (`|EnumInequality` (`self.CurrentMentalState`) "NewEnumerator1")
    (set `self.CurrentMentalState` "NewEnumerator0")
    (`self.Set Mental States in BB`)
    (return)))

(fn `StartCombat`
  (if (`|EnumInequality` (`self.CurrentMentalState`) "NewEnumerator2")
    (set `self.CurrentMentalState` "NewEnumerator0")
    (`self.Set Mental States in BB`)
    (return)))

(fn `StartNeutral`
  (if (`|EnumInequality` (`self.CurrentMentalState`) "NewEnumerator0")
    (set `self.CurrentMentalState` "NewEnumerator0")
    (`self.Set Mental States in BB`)
    (return)))

(fn `StopAlert`
  (`BlackboardComponent.ClearValue` (`self.Blackboard`) "StimulusLocation"))

(fn `StopCombat`)

(fn `StopNeutral`
  (`BlackboardComponent.ClearValue` (`self.Blackboard`) "RandomPointPatrolling"))

(fn `TempEnemySet`
  (params (TempEnemy :type "Actor Object Reference"))
  (locals (Temptarget :type "Actor Object Reference"))
  (`/Engine/EditorBlueprintResources/StandardMacros.IsValid` TempEnemy
    (:`Is Valid`
      (`BlackboardComponent.SetValueAsObject` (`self.Blackboard`) "Enemy" TempEnemy)
      (return))
    (:`Is Not Valid`
      (`self.RemoveTarget`))))

(fn `UserConstructionScript`)